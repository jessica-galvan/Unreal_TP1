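; BP_Shadow is a shadow volume that switches the player's invisibility state on entering and leaving it.
; Begin and end overlaps on its Shadow component respond only to player 0's BP_ThirdPersonCharacter.
; Entry calls the character's SetInvisibilityEvent and exit calls SetVisibleEvent, each followed by BeInvisibleEvent and accompanied by a debug print.
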(event OnComponentBeginOverlap(Shadow)
  (params (OverlappedComponent :type Primitive%20Component%20Object%20Reference) (OtherActor :type Actor%20Object%20Reference) (OtherComp :type Primitive%20Component%20Object%20Reference) (OtherBodyIndex :type Integer) (bFromSweep :type Boolean) (SweepResult :type Hit%20Result%20Structure%20%28by%20ref%29))
  (if (== OtherActor (Game|GetPlayerCharacter 0))
    (Utilities|Casting|CastToBP_ThirdPersonCharacter OtherActor)
    (Development|PrintString "PlayerInvisible")
    (bind _asbp_third_person_character (Utilities|Casting|CastToBP_ThirdPersonCharacter OtherActor))
    (Default|SetInvisibilityEvent _asbp_third_person_character)
    (Default|BeInvisibleEvent _asbp_third_person_character)))

(event OnComponentEndOverlap(Shadow)
  (params (OverlappedComponent :type Primitive%20Component%20Object%20Reference) (OtherActor :type Actor%20Object%20Reference) (OtherComp :type Primitive%20Component%20Object%20Reference) (OtherBodyIndex :type Integer))
  (if (== OtherActor (Game|GetPlayerCharacter 0))
    (Utilities|Casting|CastToBP_ThirdPersonCharacter OtherActor)
    (Development|PrintString "PlayerVisible")
    (bind _asbp_third_person_character (Utilities|Casting|CastToBP_ThirdPersonCharacter OtherActor))
    (Default|SetVisibleEvent _asbp_third_person_character)
    (Default|BeInvisibleEvent _asbp_third_person_character)))

(fn ConstructionScript)